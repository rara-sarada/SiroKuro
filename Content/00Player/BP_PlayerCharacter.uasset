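; Player character for a shooter with a black/white polarity mechanic: ChangeColor swaps material and post-process, and colored damage is either absorbed or taken based on the current color.
; GetSkill reads DT_Skill to fill active skills and stacking passives that modify walk speed and shot interval.
; Two skill slots spawn actors, teleport or apply timed buffs, calling a pod shot when flagged busy.
; AttackChecker fires rate-limited bullets, penetrating when that buff is active.
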(event Custom|GetSkill
  (params (SkillName :type String))
  (bind _passive (Variables|Default|Getpassive))
  (bind _returnvalue (Utilities|GetDataTableRow "/Game/00Player/DT_Skill.DT_Skill" (Utilities|String|StringToName SkillName))
    (:then
      (if (.Skill (Utilities|Struct|BreakF_Skill _returnvalue))
        (bind (_success _tileno) (Default|QuerySkill (Variables|Default|GetSkillSystemComponent) SkillName))
        (if (and _success (< _tileno 2))
          (Utilities|Array|Add (Variables|Default|GetSkill) (.Name (Utilities|Struct|BreakF_Skill _returnvalue))))
        (else
          (bind _success_2 (Default|QueryPassive (Variables|Default|GetSkillSystemComponent) SkillName))
          (if _success_2
            (Utilities|Map|Add _passive (.Name (Utilities|Struct|BreakF_Skill _returnvalue)) 1)
            (CallFunction|GetPassive)
            (else
              (Utilities|Map|Add _passive (.Name (Utilities|Struct|BreakF_Skill _returnvalue)) (+ (.Value (Utilities|Map|Find _passive (.Name (Utilities|Struct|BreakF_Skill _returnvalue)))) 1))
              (CallFunction|GetPassive))))))))

(event Custom|GetPassive
  (bind _charactermovement (Variables|Character|GetCharacterMovement))
  (bind _keys (Utilities|Map|Keys (Variables|Default|Getpassive)))
  (for _array_element _keys
    (switch name _array_element
      (:SpeedUP
        (Variables|/Script/Engine.CharacterMovementComponent|SetMaxWalkSpeed _charactermovement (* (Variables|/Script/Engine.CharacterMovementComponent|GetMaxWalkSpeed _charactermovement) (* (.Value (Utilities|Map|Find (Variables|Default|Getpassive) "SpeedUP")) 1.2))))
      (:ShootingSpeedUP
        (Variables|Default|SetShotTime (- (Variables|Default|GetShotTime) (* (.Value (Utilities|Map|Find (Variables|Default|Getpassive) "ShootingSpeedUP")) 0.01)))))))

(event Custom|ASkillFinCheck
  (Utilities|IsValid (stale EventUseSkillA _returnvalue_2)
    (:Is%20Not%20Valid
      (Variables|Default|SetSkillANow false)
      (Utilities|Time|ClearandInvalidateTimerbyHandle (stale EventUseSkillA _returnvalue_3)))))

(event Custom|BSkillFinCheck
  (Utilities|IsValid (stale EventUseSkillB _returnvalue_2)
    (:Is%20Not%20Valid
      (Variables|Default|SetSkillBNow false)
      (Utilities|Time|ClearandInvalidateTimerbyHandle (stale EventUseSkillB _returnvalue_3)))))

(event Game|Damage|EventAnyDamage
  (params (Damage :type Float%20%28single-precision%29) (DamageType :type Damage%20Type%20Object%20Reference) (InstigatedBy :type Controller%20Object%20Reference) (DamageCauser :type Actor%20Object%20Reference))
  (bind _returnvalue (Utilities|GetClass DamageType))
  (bind _playercolor (Variables|Default|GetPlayerColor))
  (bind _returnvalue_2 (== _returnvalue "/Game/00System/DamageType/White.White_C"))
  (bind _returnvalue_3 (== _returnvalue "/Game/00System/DamageType/Black.Black_C"))
  ;[0 0.4844 1] ダメージ処理
  (if (or _returnvalue_3 _returnvalue_2) ; クラスが設定された攻撃か判定
    (if (or (and _returnvalue_3 _playercolor) (and _returnvalue_2 (not _playercolor)))
      (Variables|Default|SetapplyAnyDamageNow true :!label _label)
      (Variables|Default|SethitPoint (Math|Float|Truncate (- (Variables|Default|GethitPoint) Damage)))
      (Development|PrintString (Utilities|String|Append "ダメージを[" (Utilities|String|ToString(Float) Damage) "]受けました"))
      (else
        (Development|PrintString "吸収")))
    (else
      (goto _label))))

(event EventChangeColor
  (bind _output_get (Variables|Default|SetPlayerColor (not (Variables|Default|GetPlayerColor))))
  (Rendering|Material|SetMaterial (Variables|Character|GetMesh) 0 (select _output_get "/Game/00Player/Mesh/M_Mesh_2.M_Mesh_2" "/Game/00Player/Mesh/M_Mesh.M_Mesh"))
  (Rendering|SetVisibility (Variables|Default|GetPostProcessA) (not (Variables|Default|GetPlayerColor)) true)
  (Rendering|SetVisibility (Variables|Default|GetPostProcessB) (Variables|Default|GetPlayerColor) false))

(event EventAttackChecker
  (bind _skillset (Variables|Default|GetSkillSet))
  (CallFunction|PrintMaster "Now Attack" (Utilities|String|ToString(Boolean) (stale _output_get)) false 5.0)
  (if (not (Variables|Default|GetNowAttack))
    (bind _output_get (Variables|Default|SetNowAttack true))
    (bind _keys (Utilities|Map|Keys _skillset))
    (for _array_element _keys
      (if (.Value (Utilities|Map|Find _skillset _array_element))
        (switch name _array_element
          (:PenetratingBullet
            (bind _returnvalue (Game|SpawnActorfromClass "/Game/00Player/BP_Bullet.BP_Bullet_C" (Math|Transform|MakeTransform (+ (Transformation|GetActorLocation) (* (Transformation|GetActorForwardVector) 100)) (Transformation|GetActorRotation) "1.000000,1.000000,1.000000") "Undefined" 0 0))
            (Variables|/Game/00Player/BP_Bullet.BP_Bullet_C|SetPenetratingBullet _returnvalue true)
            (Utilities|FlowControl|Delay (Variables|Default|GetShotTime))
            (Variables|Default|SetNowAttack false)))))
    (if (not (.Value (Utilities|Map|Find _skillset _array_element)))
      (bind _returnvalue_2 (Game|SpawnActorfromClass "/Game/00Player/BP_Bullet.BP_Bullet_C" (Math|Transform|MakeTransform (+ (Transformation|GetActorLocation) (* (Transformation|GetActorForwardVector) 100)) (Transformation|GetActorRotation) "1.000000,1.000000,1.000000") "Undefined" 0 0))
      (Variables|/Game/00Player/BP_Bullet.BP_Bullet_C|SetPenetratingBullet _returnvalue_2 false)
      (Utilities|FlowControl|Delay (Variables|Default|GetShotTime))
      (Variables|Default|SetNowAttack false))))

(event EventBeginPlay
  ;[0 1 1] 所持スキルの確認
  (|CallParentFunction)
  (for _array_element 0
    (bind _success (Default|QuerySkill (Variables|Default|GetSkillSystemComponent) _array_element))
    (if _success
      _)))

(event EventUseSkillA
  (bind _skill (Variables|Default|GetSkill))
  (if (Variables|Default|GetSkillANow)
    (Default|CallPodShot)
    (else
      (Variables|Default|SetSkillANow true)
      (if (>= (Utilities|Array|Length _skill) 1)
        (bind _returnvalue (Utilities|GetDataTableRow "/Game/00Player/DT_Skill.DT_Skill" (Utilities|Array|Get(acopy) _skill))
          (:then
            (switch name (.Name (Utilities|Struct|BreakF_Skill _returnvalue))
              (:Default
                (if (.SpawnSkill (Utilities|Struct|BreakF_Skill _returnvalue))
                  (bind _returnvalue_2 (Game|SpawnActorfromClass (.SkillActor (Utilities|Struct|BreakF_Skill _returnvalue)) (Math|Transform|MakeTransform (+ (Transformation|GetActorLocation) (* (Transformation|GetActorForwardVector) 100)) (Transformation|GetActorRotation) "1.000000,1.000000,1.000000") "Undefined" 0 0))
                  (bind _returnvalue_3 (Utilities|Time|SetTimerbyEvent (delegate Custom|ASkillFinCheck) 1.0 true))
                  (else
                    (Utilities|Map|Add (Variables|Default|GetSkillSet) (.Name (Utilities|Struct|BreakF_Skill _returnvalue)) true)
                    (Utilities|FlowControl|Delay 2.0)
                    (Utilities|Map|Add (Variables|Default|GetSkillSet) (.Name (Utilities|Struct|BreakF_Skill _returnvalue)) false)
                    (Variables|Default|SetSkillANow false))))
              (:Teleport
                (Transformation|SetActorLocation (+ (Transformation|GetActorLocation) (* (Transformation|GetActorForwardVector) 1e+02)) false true)
                (Variables|Default|SetSkillANow false))
              (:RapidFire
                (Variables|Default|SetShotTime 0.2)
                (Utilities|FlowControl|Delay 2.0)
                (Variables|Default|SetShotTime 1.0)
                (Variables|Default|SetSkillANow false))
              (:Bisection
                (Variables|Default|SetBisectionNow true)
                (Utilities|FlowControl|Delay 2.0)
                (Variables|Default|SetBisectionNow false)
                (Variables|Default|SetSkillANow false)))))))))

(event EventUseSkillB
  (bind _skill (Variables|Default|GetSkill))
  (if (Variables|Default|GetSkillBNow)
    (Default|CallPodShot)
    (elif (>= (Utilities|Array|Length _skill) 2)
      (bind _returnvalue (Utilities|GetDataTableRow "/Game/00Player/DT_Skill.DT_Skill" (Utilities|Array|Get(acopy) _skill 1))
        (:then
          (switch name (.Name (Utilities|Struct|BreakF_Skill _returnvalue))
            (:Default
              (if (.SpawnSkill (Utilities|Struct|BreakF_Skill _returnvalue))
                (bind _returnvalue_2 (Game|SpawnActorfromClass (.SkillActor (Utilities|Struct|BreakF_Skill _returnvalue)) (Math|Transform|MakeTransform (+ (Transformation|GetActorLocation) (* (Transformation|GetActorForwardVector) 100)) (Transformation|GetActorRotation) "1.000000,1.000000,1.000000") "Undefined" 0 0))
                (bind _returnvalue_3 (Utilities|Time|SetTimerbyEvent (delegate Custom|BSkillFinCheck) 1.0 true))
                (else
                  (Utilities|Map|Add (Variables|Default|GetSkillSet) (.Name (Utilities|Struct|BreakF_Skill _returnvalue)) true)
                  (Utilities|FlowControl|Delay 2.0)
                  (Utilities|Map|Add (Variables|Default|GetSkillSet) (.Name (Utilities|Struct|BreakF_Skill _returnvalue)) false)
                  (Variables|Default|SetSkillBNow false))))
            (:Teleport
              (Transformation|SetActorLocation (+ (Transformation|GetActorLocation) (* (Transformation|GetActorForwardVector) 1e+02)) false true)
              (Variables|Default|SetSkillBNow false))
            (:RapidFire
              (Variables|Default|SetShotTime 0.2)
              (Utilities|FlowControl|Delay 2.0)
              (Variables|Default|SetShotTime 1.0)
              (Variables|Default|SetSkillBNow false))
            (:Bisection
              (Variables|Default|SetBisectionNow true)
              (Utilities|FlowControl|Delay 2.0)
              (Variables|Default|SetBisectionNow false)
              (Variables|Default|SetSkillBNow false))))))))

(fn ConstructionScript)