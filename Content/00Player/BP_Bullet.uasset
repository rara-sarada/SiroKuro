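; BP_Bullet is a bullet actor that damages whatever actor its sphere component overlaps.
; On BeginPlay it sets the sphere's material from the player character's state: a mannequin body material while BisectionNow is set, otherwise material A or B according to PlayerColor.
; On overlap it applies a fixed amount of damage and destroys itself unless its PenetratingBullet flag is set.
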(event OnComponentBeginOverlap(Sphere)
  (params (OverlappedComponent :type Primitive%20Component%20Object%20Reference) (OtherActor :type Actor%20Object%20Reference) (OtherComp :type Primitive%20Component%20Object%20Reference) (OtherBodyIndex :type Integer) (bFromSweep :type Boolean) (SweepResult :type Hit%20Result%20Structure%20%28by%20ref%29))
  (Game|Damage|ApplyDamage OtherActor 1.0 0 0)
  (if (not (Variables|Default|GetPenetratingBullet))
    (Actor|DestroyActor)))

(event EventBeginPlay
  (bind _returnvalue (Game|GetPlayerCharacter 0))
  (bind _asbp_player_character (Utilities|Casting|CastToBP_PlayerCharacter _returnvalue))
  (if (Variables|/Game/00Player/BP_PlayerCharacter.BP_PlayerCharacter_C|GetBisectionNow _asbp_player_character)
    (Rendering|Material|SetMaterial (Variables|Default|GetSphere) 0 "/Game/Characters/Mannequin_UE4/Materials/M_MannequinUE4_Body.M_MannequinUE4_Body")
    (else
      (Rendering|Material|SetMaterial (Variables|Default|GetSphere) 0 (select (Variables|/Game/00Player/BP_PlayerCharacter.BP_PlayerCharacter_C|GetPlayerColor _asbp_player_character) "/Game/00Player/M_PlayerB.M_PlayerB" "/Game/00Player/M_PlayerA.M_PlayerA")))))

(fn ConstructionScript)