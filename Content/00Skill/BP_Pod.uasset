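; BP_Pod is a short-lived companion pod that hovers at a fixed offset from the player, fires at enemies, then destroys itself after a delay.
; On spawn it binds Shot to the player's PodShot event and picks the BP_enemyMaster nearest the player.
; Tick keeps it in position and rescans for the nearest enemy only when the cached target becomes invalid.
; Each Shot turns it toward that target and spawns a BP_Bullet ahead.
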(event Custom|Shot
  (Utilities|IsValid (Variables|Default|GetMinDistanceActor)
    (:Is%20Valid
      (Transformation|SetActorRotation (Math|Rotator|FindLookatRotation (Transformation|GetActorLocation) (Transformation|GetActorLocation (Variables|Default|GetMinDistanceActor))))
      (Game|SpawnActorfromClass "/Game/00Player/BP_Bullet.BP_Bullet_C" (Math|Transform|MakeTransform (+ (Transformation|GetActorLocation) (* (Transformation|GetActorForwardVector) 100)) (Transformation|GetActorRotation) "1.000000,1.000000,1.000000") "Undefined" 0 0))))

(event EventBeginPlay
  (bind _asbp_player_character (Utilities|Casting|CastToBP_PlayerCharacter (Game|GetPlayerCharacter 0)))
  (EventDispatchers|BindEventtoPodShot _asbp_player_character (delegate Custom|Shot))
  (bind _outactors (Actor|GetAllActorsOfClass "/Game/00Enemy/BP_enemyMaster.BP_enemyMaster_C"))
  (for (_array_element _array_index) _outactors
    (if (== _array_index 0)
      (Variables|Default|SetMinDistance (Transformation|GetDistanceTo _array_element (Game|GetPlayerCharacter 0)))
      (Variables|Default|SetMinDistanceActor _array_element)
      (elif (< (Transformation|GetDistanceTo _array_element (Game|GetPlayerCharacter 0)) (Variables|Default|GetMinDistance))
        (Variables|Default|SetMinDistance (Transformation|GetDistanceTo _array_element (Game|GetPlayerCharacter 0)))
        (Variables|Default|SetMinDistanceActor _array_element))))
  (Utilities|FlowControl|Delay 1e+01)
  (Actor|DestroyActor))

(event EventTick
  (params (DeltaSeconds :type Float%20%28single-precision%29))
  (Transformation|SetActorLocation (+ (Transformation|GetActorLocation (Game|GetPlayerCharacter 0)) "100.000000,0,0") false false)
  (Utilities|IsValid (Variables|Default|GetMinDistanceActor)
    (:Is%20Not%20Valid
      (bind _outactors (Actor|GetAllActorsOfClass "/Game/00Enemy/BP_enemyMaster.BP_enemyMaster_C"))
      (for (_array_element _array_index) _outactors
        (if (== _array_index 0)
          (Variables|Default|SetMinDistance (Transformation|GetDistanceTo _array_element (Game|GetPlayerCharacter 0)))
          (Variables|Default|SetMinDistanceActor _array_element)
          (elif (< (Transformation|GetDistanceTo _array_element (Game|GetPlayerCharacter 0)) (Variables|Default|GetMinDistance))
            (Variables|Default|SetMinDistance (Transformation|GetDistanceTo _array_element (Game|GetPlayerCharacter 0)))
            (Variables|Default|SetMinDistanceActor _array_element)))))))

(fn ConstructionScript)