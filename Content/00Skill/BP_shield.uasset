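; BP_shield is a color-dependent shield skill actor that destroys bullets touching its Cube.
; On BeginPlay it copies the player character's boolean PlayerColor and gives the Cube the matching player material, A or B.
; On overlap it gets the other actor's color code through BulletColorMessage and destroys that actor only when the code pairs with the stored color.
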(event OnComponentBeginOverlap(Cube)
  (params (OverlappedComponent :type Primitive%20Component%20Object%20Reference) (OtherActor :type Actor%20Object%20Reference) (OtherComp :type Primitive%20Component%20Object%20Reference) (OtherBodyIndex :type Integer) (bFromSweep :type Boolean) (SweepResult :type Hit%20Result%20Structure%20%28by%20ref%29))
  (bind _color (Class|BIBulletColor|BulletColor(Message) OtherActor))
  (if (Variables|Default|GetPlayer%20Color)
    (if (== _color 1)
      (Actor|DestroyActor OtherActor))
    (elif (== _color 2)
      (Actor|DestroyActor OtherActor))))

(event EventBeginPlay
  (bind _returnvalue (Game|GetPlayerCharacter 0))
  (bind _asbp_player_character (Utilities|Casting|CastToBP_PlayerCharacter _returnvalue))
  (bind _playercolor (Variables|/Game/00Player/BP_PlayerCharacter.BP_PlayerCharacter_C|GetPlayerColor _asbp_player_character))
  (Variables|Default|SetPlayer%20Color _playercolor)
  (Rendering|Material|SetMaterial (Variables|Default|GetCube) 0 (select _playercolor "/Game/00Player/M_PlayerB.M_PlayerB" "/Game/00Player/M_PlayerA.M_PlayerA")))

(fn ConstructionScript)