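; BP_HomingRocket is a homing projectile that chases an enemy and deals damage on contact.
; On BeginPlay it sets its sphere material from the player's bisection and color state, then picks the BP_enemyMaster nearest the player as its fixed target.
; Each Tick it turns toward that target and steps forward a fixed, frame-rate-dependent distance.
; Sphere1 overlap damages whatever actor it touches, then destroys the rocket.
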(event OnComponentBeginOverlap(Sphere1)
  (params (OverlappedComponent :type Primitive%20Component%20Object%20Reference) (OtherActor :type Actor%20Object%20Reference) (OtherComp :type Primitive%20Component%20Object%20Reference) (OtherBodyIndex :type Integer) (bFromSweep :type Boolean) (SweepResult :type Hit%20Result%20Structure%20%28by%20ref%29))
  (Game|Damage|ApplyDamage OtherActor 1.0 0 0)
  (Actor|DestroyActor))

(event EventBeginPlay
  (bind _returnvalue (Game|GetPlayerCharacter 0))
  (bind _asbp_player_character (Utilities|Casting|CastToBP_PlayerCharacter _returnvalue))
  (if (Variables|/Game/00Player/BP_PlayerCharacter.BP_PlayerCharacter_C|GetBisectionNow _asbp_player_character)
    (Rendering|Material|SetMaterial (Variables|Default|GetSphere) 0 "/Game/Characters/Mannequins/Materials/M_Mannequin.M_Mannequin")
    (else
      (Rendering|Material|SetMaterial (Variables|Default|GetSphere) 0 (select (Variables|/Game/00Player/BP_PlayerCharacter.BP_PlayerCharacter_C|GetPlayerColor _asbp_player_character) "/Game/00Player/M_PlayerB.M_PlayerB" "/Game/00Player/M_PlayerA.M_PlayerA"))))
  (bind _outactors (Actor|GetAllActorsOfClass "/Game/00Enemy/BP_enemyMaster.BP_enemyMaster_C"))
  (for (_array_element _array_index) _outactors
    (if (== _array_index 0)
      (Variables|Default|SetMinDistance (Transformation|GetDistanceTo _array_element (Game|GetPlayerCharacter 0)))
      (Variables|Default|SetMinDistanceActor _array_element)
      (elif (< (Transformation|GetDistanceTo _array_element (Game|GetPlayerCharacter 0)) (Variables|Default|GetMinDistance))
        (Variables|Default|SetMinDistanceActor _array_element)
        (Variables|Default|SetMinDistance (Transformation|GetDistanceTo _array_element (Game|GetPlayerCharacter 0)))))))

(event Collision|EventActorBeginOverlap
  (params (OtherActor :type Actor%20Object%20Reference)))

(event EventTick
  (params (DeltaSeconds :type Float%20%28single-precision%29))
  (Transformation|SetActorRotation (Math|Rotator|FindLookatRotation (Transformation|GetActorLocation) (Transformation|GetActorLocation (Variables|Default|GetMinDistanceActor))))
  (Transformation|SetActorLocation (+ (Transformation|GetActorLocation) (* (Transformation|GetActorForwardVector) 1e+01)) false false))

(fn ConstructionScript)