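; Sniper enemy in one of two color variants, chosen by EnemyColor0, which turns to face the player every tick.
; Shot shows a color-matched Niagara laser pointer that follows the player through a fast looping timer.
; After a delay it locks aim by stopping tick and the timer, then briefly pauses, clears the laser and fires the matching sniper bullet from Arrow1 before resuming tracking.
; Damage handling is left to the parent class.
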(event Custom|LaserPointerPos
  (Niagara|SetNiagaraVariable(Vector3) (Variables|Default|GetNS_LaserPointer) "PlayerVector" (Transformation|GetActorLocation (Game|Player|GetPlayerPawn 0))))

(event Custom|Shot
  (bind _arrow1 (Variables|Default|GetArrow1))
  (bind _ns_laserpointer (Variables|Default|GetNS_LaserPointer))
  (bind _arrow1_2 (Variables|Default|GetArrow1))
  (bind _ns_laserpointer_2 (Variables|Default|GetNS_LaserPointer))
  (Niagara|SetNiagaraVariable(Vector3) (Variables|Default|GetNS_LaserPointer) "PlayerVector" (Transformation|GetActorLocation))
  (Niagara|SetNiagaraVariable(Vector3) _ns_laserpointer "PlayerVector" (Transformation|GetActorLocation (Game|Player|GetPlayerPawn 0)))
  (bind _returnvalue (Utilities|Time|SetTimerbyEvent (delegate Custom|LaserPointerPos) 0.01 true))
  (Variables|Default|SetLaserTimer _returnvalue)
  (if (Variables|Default|GetEnemyColor_0)
    (Class|NiagaraComponent|SetAsset _ns_laserpointer "/Game/00Enemy/Enemy4/NS_LaserPointerA.NS_LaserPointerA" true)
    (else
      (Class|NiagaraComponent|SetAsset _ns_laserpointer "/Game/00Enemy/Enemy4/NS_LaserPointerB.NS_LaserPointerB" true)))
  (Utilities|FlowControl|Delay 3.0)
  (Variables|Default|SetPlayerLocation (Transformation|GetActorLocation (Game|Player|GetPlayerPawn 0)))
  (Actor|Tick|SetActorTickEnabled false)
  (Utilities|Time|ClearandInvalidateTimerbyHandle (Variables|Default|GetLaserTimer))
  (Utilities|FlowControl|Delay 0.3)
  (if (Variables|Default|GetEnemyColor_0)
    (Class|NiagaraComponent|SetAsset _ns_laserpointer_2 0 true)
    (Game|SpawnActorfromClass "/Game/00Enemy/BP_enemySniperBulletA.BP_enemySniperBulletA_C" (Math|Transform|MakeTransform (Transformation|GetWorldLocation _arrow1_2) (Transformation|GetWorldRotation _arrow1_2) "1.000000,1.000000,1.000000") "Undefined" 0 0)
    (else
      (Class|NiagaraComponent|SetAsset _ns_laserpointer_2 0 true)
      (Game|SpawnActorfromClass "/Game/00Enemy/BP_enemySniperBulletB.BP_enemySniperBulletB_C" (Math|Transform|MakeTransform (Transformation|GetWorldLocation _arrow1) (Transformation|GetWorldRotation _arrow1) "1.000000,1.000000,1.000000") "Undefined" 0 0)))
  (Actor|Tick|SetActorTickEnabled true))

(event EventBeginPlay
  (bind _cube (Variables|Default|GetCube))
  (if (Variables|Default|GetEnemyColor_0)
    (Rendering|Material|SetMaterial _cube 0 "/Game/00Player/M_PlayerA.M_PlayerA")
    (else
      (Rendering|Material|SetMaterial _cube 0 "/Game/00Player/M_PlayerB.M_PlayerB"))))

(event Collision|EventActorBeginOverlap
  (params (OtherActor :type Actor%20Object%20Reference)))

(event EventTick
  (params (DeltaSeconds :type Float%20%28single-precision%29))
  (Transformation|SetActorRotation (Math|Rotator|FindLookatRotation (Transformation|GetActorLocation) (Transformation|GetActorLocation (Game|GetPlayerCharacter 0)))))

(event Game|Damage|EventAnyDamage
  (params (Damage :type Float%20%28single-precision%29) (DamageType :type Damage%20Type%20Object%20Reference) (InstigatedBy :type Controller%20Object%20Reference) (DamageCauser :type Actor%20Object%20Reference))
  (|CallParentFunction Damage DamageType InstigatedBy DamageCauser))

(fn ConstructionScript)