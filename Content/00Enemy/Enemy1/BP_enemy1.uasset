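; BP_enemy1 is a two-color enemy that turns to face the player and fires bullets of a type matching its color.
; On BeginPlay, EnemyColor0 selects a white or black material for its two cubes.
; Tick rotates the actor toward player 0, and the Shot event spawns BP_enemyBulletA or BP_enemyBulletB at Arrow1 according to that same flag.
; Damage and attack-area hits are passed straight to the parent class.
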(event Custom|Shot
  (bind _arrow1 (Variables|Default|GetArrow1))
  (bind _arrow1_2 (Variables|Default|GetArrow1))
  (if (Variables|Default|GetEnemyColor_0)
    (Game|SpawnActorfromClass "/Game/00Enemy/BP_enemyBulletA.BP_enemyBulletA_C" (Math|Transform|MakeTransform (Transformation|GetWorldLocation _arrow1_2) (Transformation|GetWorldRotation _arrow1_2) "1.000000,1.000000,1.000000") "Undefined" 0 0)
    (else
      (Game|SpawnActorfromClass "/Game/00Enemy/BP_enemyBulletB.BP_enemyBulletB_C" (Math|Transform|MakeTransform (Transformation|GetWorldLocation _arrow1) (Transformation|GetWorldRotation _arrow1) "1.000000,1.000000,1.000000") "Undefined" 0 0))))

(event Collision|EventActorBeginOverlap
  (params (OtherActor :type Actor%20Object%20Reference)))

(event Game|Damage|EventAnyDamage
  (params (Damage :type Float%20%28single-precision%29) (DamageType :type Damage%20Type%20Object%20Reference) (InstigatedBy :type Controller%20Object%20Reference) (DamageCauser :type Actor%20Object%20Reference))
  (|CallParentFunction Damage DamageType InstigatedBy DamageCauser))

(event EventHitAttackArea
  (params (NowHit :type Boolean))
  (|CallParentFunction NowHit))

(event EventTick
  (params (DeltaSeconds :type Float%20%28single-precision%29))
  (|CallParentFunction DeltaSeconds)
  (Transformation|SetActorRotation (Math|Rotator|FindLookatRotation (Transformation|GetActorLocation) (Transformation|GetActorLocation (Game|GetPlayerCharacter 0)))))

(event EventBeginPlay
  (bind _cube (Variables|Default|GetCube))
  (|CallParentFunction)
  (if (Variables|Default|GetEnemyColor_0)
    (Rendering|Material|SetMaterial _cube 0 "/Game/00Enemy/Material/M_White.M_White")
    (else
      (Rendering|Material|SetMaterial _cube 0 "/Game/00Enemy/Material/M_Black.M_Black"))))

(fn ConstructionScript)