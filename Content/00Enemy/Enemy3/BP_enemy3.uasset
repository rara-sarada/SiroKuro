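; BP_enemy3 is an enemy that faces the player and fires a five-way bullet fan when its Shot event runs.
; EnemyColor0 sets its two cubes to white or black on BeginPlay and selects bullet type A or B.
; Tick turns it toward the player every frame, and Shot spawns the evenly yaw-spaced spread from Arrow1.
; Damage is passed straight to the parent class.
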(event Custom|Shot
  (bind _arrow1 (Variables|Default|GetArrow1))
  (bind _arrow1_2 (Variables|Default|GetArrow1))
  (if (Variables|Default|GetEnemyColor_0)
    (for _index (range -2 2)
      (Game|SpawnActorfromClass "/Game/00Enemy/BP_enemyBulletA.BP_enemyBulletA_C" (Math|Transform|MakeTransform (Transformation|GetWorldLocation _arrow1_2) (Math|Rotator|CombineRotators (Transformation|GetWorldRotation _arrow1_2) (Math|Rotator|MakeRotator 0.0 0.0 (* _index 2e+01))) "1.000000,1.000000,1.000000") "Undefined" 0 0))
    (else
      (for _index_2 (range -2 2)
        (Game|SpawnActorfromClass "/Game/00Enemy/BP_enemyBulletB.BP_enemyBulletB_C" (Math|Transform|MakeTransform (Transformation|GetWorldLocation _arrow1) (Math|Rotator|CombineRotators (Transformation|GetWorldRotation _arrow1) (Math|Rotator|MakeRotator 0.0 0.0 (* _index_2 2e+01))) "1.000000,1.000000,1.000000") "Undefined" 0 0)))))

(event EventBeginPlay
  (bind _cube (Variables|Default|GetCube))
  (if (Variables|Default|GetEnemyColor_0)
    (Rendering|Material|SetMaterial _cube 0 "/Game/00Enemy/Material/M_White.M_White")
    (else
      (Rendering|Material|SetMaterial _cube 0 "/Game/00Enemy/Material/M_Black.M_Black"))))

(event Collision|EventActorBeginOverlap
  (params (OtherActor :type Actor%20Object%20Reference)))

(event EventTick
  (params (DeltaSeconds :type Float%20%28single-precision%29))
  (Transformation|SetActorRotation (Math|Rotator|FindLookatRotation (Transformation|GetActorLocation) (Transformation|GetActorLocation (Game|GetPlayerCharacter 0)))))

(event Game|Damage|EventAnyDamage
  (params (Damage :type Float%20%28single-precision%29) (DamageType :type Damage%20Type%20Object%20Reference) (InstigatedBy :type Controller%20Object%20Reference) (DamageCauser :type Actor%20Object%20Reference))
  (|CallParentFunction Damage DamageType InstigatedBy DamageCauser))

(fn ConstructionScript)