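; BP_enemyMaster is an enemy Blueprint, by name the master class, that takes periodic damage while inside an attack area.
; HitAttackArea sets a flag that Tick polls, using a DoOnce to start a looping self-damage timer and clearing it on exit.
; AnyDamage negates HP rather than subtracting Damage, then destroys the actor at zero or below.
; On destruction it notifies GM_GamePlay through DestroyEnemy.
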(event Custom|AreaDamage
  (Game|Damage|ApplyDamage self 1.0 0 0)
  (Development|PrintString (Utilities|String|ToString(Float) (Variables|Default|GetHP))))

(event EventDestroyEnemy)

(event Collision|EventActorBeginOverlap
  (params (OtherActor :type Actor%20Object%20Reference)))

(event EventTick
  (params (DeltaSeconds :type Float%20%28single-precision%29))
  (if (Variables|Default|GetInAttackArea)
    (Utilities|FlowControl|DoOnce false :!label _label
      (:Completed
        (bind _returnvalue (Utilities|Time|SetTimerbyEvent (delegate Custom|AreaDamage) 5.0 true))))
    (else
      (Utilities|Time|ClearandInvalidateTimerbyHandle _returnvalue)
      (goto _label Reset))))

(event Game|Damage|EventAnyDamage
  (params (Damage :type Float%20%28single-precision%29) (DamageType :type Damage%20Type%20Object%20Reference) (InstigatedBy :type Controller%20Object%20Reference) (DamageCauser :type Actor%20Object%20Reference))
  (|CallParentFunction Damage DamageType InstigatedBy DamageCauser)
  (Variables|Default|SetHP (- 0.0 (Variables|Default|GetHP)))
  (if (<= (Variables|Default|GetHP) 0.0)
    (Actor|DestroyActor)))

(event EventDestroyed
  (|CallParentFunction)
  (bind _asgm_game_play (Utilities|Casting|CastToGM_GamePlay (Game|GetGameMode)))
  (Default|DestroyEnemy _asgm_game_play))

(event EventHitAttackArea
  (params (NowHit :type Boolean))
  (Variables|Default|SetInAttackArea NowHit))

(fn ConstructionScript)