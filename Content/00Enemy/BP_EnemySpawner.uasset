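; BP_EnemySpawner is a spawn point that creates one of four enemy types on demand at its own transform.
; Its EnemySpawn event switches on the given enemy name and spawns the matching pawn class with its own behavior tree.
; The construction script colors the Sphere component by PopType (Atype or Btype) through a material choice.
; The spawner does not trigger itself, as BeginPlay, overlap and Tick are empty.
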(event Custom|EnemySpawn
  (params (Enemyname :type Enum_EnemyType%20Enum :default "NewEnumerator0"))
  (bind _returnvalue (Transformation|GetActorTransform))
  (bind _returnvalue_2 (Transformation|GetActorTransform))
  (bind _returnvalue_3 (Transformation|GetActorTransform))
  (bind _returnvalue_4 (Transformation|GetActorTransform))
  (switch Utilities|FlowControl|Switch|SwitchonEnum_EnemyType Enemyname
    (:NewEnumerator0
      (AI|SpawnAIFromClass "/Game/00Enemy/Enemy1/BP_enemy1.BP_enemy1_C" "/Game/00Enemy/Enemy1/BT_enemy1.BT_enemy1" (.location _returnvalue_3) (.rotation _returnvalue_3) false 0))
    (:NewEnumerator1
      (AI|SpawnAIFromClass "/Game/00Enemy/Enemy2/BP_enemy2.BP_enemy2_C" "/Game/00Enemy/Enemy2/BT_enemy2.BT_enemy2" (.location _returnvalue_4) (.rotation _returnvalue_4) false 0))
    (:NewEnumerator2
      (AI|SpawnAIFromClass "/Game/00Enemy/Enemy3/BP_enemy3.BP_enemy3_C" "/Game/00Enemy/Enemy3/BT_enemy3.BT_enemy3" (.location _returnvalue) (.rotation _returnvalue) false 0))
    (:NewEnumerator3
      (AI|SpawnAIFromClass "/Game/00Enemy/Enemy4/BP_enemy4.BP_enemy4_C" "/Game/00Enemy/Enemy4/BT_enemy4.BT_enemy4" (.location _returnvalue_2) (.rotation _returnvalue_2) false 0))))

(event EventBeginPlay)

(event Collision|EventActorBeginOverlap
  (params (OtherActor :type Actor%20Object%20Reference)))

(event EventTick
  (params (DeltaSeconds :type Float%20%28single-precision%29)))

(fn ConstructionScript
  (Rendering|Material|SetMaterial (Variables|Default|GetSphere) 0 (Utilities|Select :Index (Variables|Default|GetPopType) :NewEnumerator0 "/Game/00Enemy/Any/M_SpawnA.M_SpawnA" :NewEnumerator1 "/Game/00Enemy/Any/M_SpawnB.M_SpawnB")))