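; Map-maker component that builds the floor layout of a stage from its row in DT_FloorSetting.
; MakeMap uses the Percent helper on map values to choose a key for the floor count, then resizes FloorStructure to that depth.
; It repeats the same values-to-key pick for each NumberOfLevel entry, writing that floor's room count into FloorStructure.
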(event Custom|MakeMap
  (params (StageX :type Name))
  (bind _returnvalue (Utilities|GetDataTableRow "/Game/00System/MapMaker/DataTable/DT_FloorSetting.DT_FloorSetting" StageX)
    (:then
      (bind _output_get (Variables|Default|SetMapSetting _returnvalue))
      (bind _values (Utilities|Map|Values (.FloorCount (Utilities|Struct|BreakST_FloorSetting _output_get))))
      (bind _arrayindex (CallFunction|Percent _values))
      (bind _keys (Utilities|Map|Keys (.FloorCount (Utilities|Struct|BreakST_FloorSetting _output_get))))
      (Utilities|Array|Resize (Variables|Default|GetFloorStructure) (Utilities|Array|Get(acopy) _keys _arrayindex)) ; 階層の深さを設定
      (for (_array_element _array_index) (.numberoflevel (Variables|Default|GetMapSetting))
        (bind _values_2 (Utilities|Map|Values (Utilities|Struct|BreakST_NumberOfLevel _array_element)))
        (bind _arrayindex_2 (CallFunction|Percent _values_2))
        (bind _keys_2 (Utilities|Map|Keys (Utilities|Struct|BreakST_NumberOfLevel _array_element)))
        (Utilities|Array|SetArrayElem (Variables|Default|GetFloorStructure) _array_index (Utilities|Array|Get(acopy) _keys_2 _arrayindex_2)) ; フロアごとの部屋数を設定
      ))))

(event EventBeginPlay)