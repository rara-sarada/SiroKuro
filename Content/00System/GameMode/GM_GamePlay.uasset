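; Gameplay GameMode that spawns an enemy wave for the level selected in MyGameInstance and tracks its clearing.
; After BeginPlay it gathers spawners of one random pop type and loads the level's row from DT_LevelData.
; A re-entrant event loop spends the wave's point budget on random enemies costed by Data_EnemySetting, using each spawner once.
; DestroyEnemy decrements the count and triggers the player UI's wave-clear at zero; only wave 0 is started here.
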(event Custom|WaveClear
  (bind _aspc_player (Utilities|Casting|CastToPC_Player (Game|GetPlayerController 0)))
  (Default|WaveClear (Variables|/Game/00Player/PC_Player.PC_Player_C|GetUIMaster _aspc_player)))

(event Custom|PopStart
  ;[0.2422 1 0] スポーンの処理
  (Utilities|FlowControl|Sequence
    (:then_0
      (Utilities|Array|Clear (Variables|Default|GetspawnerStanding)) ; spawnnerの初期化
      ;;[1 0 0.01897 1 12] ※必ず[Enum_PopType]の数と同数にすること
      (Variables|Default|SetpopType (Math|Conversions|ToByte(Integer) (Math|Random|RandomIntegerinRange 0 1)))
      ;;[0 0.7656 1] このWaveで使用するSpawnnerを格納
      (for _array_element (Variables|Default|GetspawnerBase)
        (if (Utilities|Enum|Equal(Enum) (Variables|/Game/00Enemy/BP_EnemySpawner.BP_EnemySpawner_C|GetPopType _array_element) (Utilities|Enum|ByteToEnumEnum_PopType (Variables|Default|GetpopType)))
          (Utilities|Array|Add (Variables|Default|GetspawnerStanding) _array_element))))
    (:then_1
      (bind _outrownames (DataTable|GetDataTableRowNames "/Game/00System/PopSystem/DT_LevelData.DT_LevelData"))
      (bind _array_element_2 (Utilities|Array|ForEachLoopwithBreak _outrownames :!label _label)
        (:LoopBody
          (bind _returnvalue (Utilities|GetDataTableRow "/Game/00System/PopSystem/DT_LevelData.DT_LevelData" _array_element_2)
            (:then
              (if (Utilities|Enum|Equal(Enum) (Variables|Default|GetenumLevelData) (.Level (Utilities|Struct|BreakST_LevelData _returnvalue)))
                (Utilities|FlowControl|Sequence
                  (:then_0
                    (Variables|Default|SetstLevelData _returnvalue)
                    (CallFunction|PopEvent))
                  (:then_1
                    (goto _label Break)))))
            (:RowNotFound
              (Development|PrintString "DT_LevelDataのリストで見つかりませんでした"))))))))

(event Custom|PopEvent
  (params (waveCount :type Integer))
  (bind _spawnerstanding (Variables|Default|GetspawnerStanding))
  (bind _outitem (Utilities|Array|Random _spawnerstanding))
  ;[0.2422 1 0] スポーンの処理
  (Variables|Default|SetwaveCount waveCount)
  (Variables|Default|SetremainingPoint (Utilities|Array|Get(acopy) (.WavePoint (Utilities|Struct|BreakST_LevelData (Variables|Default|GetstLevelData))) (Variables|Default|GetwaveCount)))
  (if (and (!= (Utilities|Array|Length (Variables|Default|GetspawnerStanding)) 0) (> (Variables|Default|GetremainingPoint) 0))
    (bind _output_get (Variables|Default|SetSpawnEnemy (.OutItem (Utilities|Array|Random (.popenemy (Utilities|Array|Get(acopy) (.SpawnVariation (Utilities|Struct|BreakST_LevelData (Variables|Default|GetstLevelData))) (Variables|Default|GetwaveCount)))))))
    (Development|PrintString (Utilities|String|Append "スポーンする敵 / " (Utilities|String|EnumtoString _output_get)) true true "(R=0.000000,G=0.660000,B=1.000000,A=1.000000)" 1e+01)
    (bind _outrownames (DataTable|GetDataTableRowNames "/Game/00Enemy/Any/Data_EnemySetting.Data_EnemySetting"))
    (bind _array_element (Utilities|Array|ForEachLoopwithBreak _outrownames :!label _label)
      (:LoopBody
        (bind _returnvalue (Utilities|GetDataTableRow "/Game/00Enemy/Any/Data_EnemySetting.Data_EnemySetting" _array_element)
          (:then
            (if (Utilities|Enum|Equal(Enum) (Variables|Default|GetSpawnEnemy) (.type _returnvalue))
              (Utilities|FlowControl|Sequence
                (:then_0
                  (if (not (< (- (Variables|Default|GetremainingPoint) (.enemypoint _returnvalue)) 0))
                    (Variables|Default|SetremainingPoint (- (Variables|Default|GetremainingPoint) (.enemypoint _returnvalue)))
                    (Math|Integer|IncrementInt (Variables|Default|GetenemyCount)
                      (:%20%20
                        (Utilities|IsValid _outitem
                          (:Is%20Valid
                            (bind _output_get_2 (Variables|Default|SetrandomSpawner _outitem))
                            (Default|EnemySpawn _output_get_2 (.type _returnvalue))
                            (Utilities|Array|RemoveItem _spawnerstanding _output_get_2)
                            (CallFunction|SpawnLoop))
                          (:Is%20Not%20Valid
                            (Development|PrintString "召喚可能するためのスポナーが足りません")))))))
                (:then_1
                  (goto _label Break)))))
          (:RowNotFound
            (Development|PrintString "DT_EnemySettingのリストで見つかりませんでした")))))
    (else
      (Development|PrintString (Utilities|String|Append "スポーンループ終了" "" (Utilities|String|ToString(Integer) (Variables|Default|GetremainingPoint))) true true "(R=0.000000,G=0.660000,B=1.000000,A=1.000000)" 1e+01)
      (Development|PrintString (Utilities|String|Append "enemy count" (Utilities|String|ToString(Integer) (Variables|Default|GetenemyCount))) true true "(R=0.000000,G=0.660000,B=1.000000,A=1.000000)" 1e+01))))

(event Custom|spawnLoop
  (bind _spawnerstanding (Variables|Default|GetspawnerStanding))
  (bind _outitem (Utilities|Array|Random _spawnerstanding))
  ;[0.2422 1 0] スポーンの処理
  (if (and (!= (Utilities|Array|Length (Variables|Default|GetspawnerStanding)) 0) (> (Variables|Default|GetremainingPoint) 0))
    (bind _output_get (Variables|Default|SetSpawnEnemy (.OutItem (Utilities|Array|Random (.popenemy (Utilities|Array|Get(acopy) (.SpawnVariation (Utilities|Struct|BreakST_LevelData (Variables|Default|GetstLevelData))) (Variables|Default|GetwaveCount)))))))
    (Development|PrintString (Utilities|String|Append "スポーンする敵 / " (Utilities|String|EnumtoString _output_get)) true true "(R=0.000000,G=0.660000,B=1.000000,A=1.000000)" 1e+01)
    (bind _outrownames (DataTable|GetDataTableRowNames "/Game/00Enemy/Any/Data_EnemySetting.Data_EnemySetting"))
    (bind _array_element (Utilities|Array|ForEachLoopwithBreak _outrownames :!label _label)
      (:LoopBody
        (bind _returnvalue (Utilities|GetDataTableRow "/Game/00Enemy/Any/Data_EnemySetting.Data_EnemySetting" _array_element)
          (:then
            (if (Utilities|Enum|Equal(Enum) (Variables|Default|GetSpawnEnemy) (.type _returnvalue))
              (Utilities|FlowControl|Sequence
                (:then_0
                  (if (not (< (- (Variables|Default|GetremainingPoint) (.enemypoint _returnvalue)) 0))
                    (Variables|Default|SetremainingPoint (- (Variables|Default|GetremainingPoint) (.enemypoint _returnvalue)))
                    (Math|Integer|IncrementInt (Variables|Default|GetenemyCount)
                      (:%20%20
                        (Utilities|IsValid _outitem
                          (:Is%20Valid
                            (bind _output_get_2 (Variables|Default|SetrandomSpawner _outitem))
                            (Default|EnemySpawn _output_get_2 (.type _returnvalue))
                            (Utilities|Array|RemoveItem _spawnerstanding _output_get_2)
                            (CallFunction|SpawnLoop))
                          (:Is%20Not%20Valid
                            (Development|PrintString "召喚可能するためのスポナーが足りません")))))))
                (:then_1
                  (goto _label Break)))))
          (:RowNotFound
            (Development|PrintString "DT_EnemySettingのリストで見つかりませんでした")))))
    (else
      (Development|PrintString (Utilities|String|Append "スポーンループ終了" "" (Utilities|String|ToString(Integer) (Variables|Default|GetremainingPoint))) true true "(R=0.000000,G=0.660000,B=1.000000,A=1.000000)" 1e+01)
      (Development|PrintString (Utilities|String|Append "enemy count" (Utilities|String|ToString(Integer) (Variables|Default|GetenemyCount))) true true "(R=0.000000,G=0.660000,B=1.000000,A=1.000000)" 1e+01))))

(event EventBeginPlay
  (Utilities|FlowControl|Sequence
    (:then_0
      (bind _outactors (Actor|GetAllActorsOfClass "/Game/00Enemy/BP_EnemySpawner.BP_EnemySpawner_C"))
      (Variables|Default|SetspawnerBase _outactors)
      (bind _asmy_game_instance (Utilities|Casting|CastToMyGameInstance (Game|GetGameInstance)))
      (Variables|Default|SetenumLevelData (Variables|/Game/00System/GameMode/MyGameInstance.MyGameInstance_C|GetEnumLevelData _asmy_game_instance)))
    (:then_1
      (bind _outrownames (DataTable|GetDataTableRowNames "/Game/00Enemy/Any/Data_EnemySetting.Data_EnemySetting"))
      (Variables|Default|SetenemynameList _outrownames))
    (:then_2
      (Utilities|FlowControl|Delay 1.0)
      (CallFunction|PopStart))))

(event EventTick
  (params (DeltaSeconds :type Float%20%28single-precision%29))
  ;[0.2422 1 0] スポーンの処理
)

(event EventDestroyEnemy
  (bind _result (Math|Integer|DecrementInt (Variables|Default|GetenemyCount))
    (:%20%20
      (if (== _result 0)
        (Development|PrintString "Wave Clear")
        (CallFunction|WaveClear)))))

(fn ConstructionScript)